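; BP_HealthChangeVolume is a box volume that periodically changes the health of a side-scroller character inside it.
; Box overlap events cast to SideScrollerCharacter, storing the reference on entry and toggling an in-volume flag on entry and exit.
; While flagged, Tick runs a Delay of HPChangeDelay, then adds ChangeInHealth to PlayerHealth, without clamping.
; A pending Delay still applies its change after the character leaves.
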(event OnComponentBeginOverlap(Box)
  (params (OverlappedComponent :type Primitive%20Component%20Object%20Reference) (OtherActor :type Actor%20Object%20Reference) (OtherComp :type Primitive%20Component%20Object%20Reference) (OtherBodyIndex :type Integer) (bFromSweep :type Boolean) (SweepResult :type Hit%20Result%20Structure%20%28by%20ref%29))
  (bind _asside_scroller_character (Utilities|Casting|CastToSideScrollerCharacter OtherActor))
  (Variables|Default|SetCharacterInVolume true))

(event OnComponentEndOverlap(Box)
  (params (OverlappedComponent :type Primitive%20Component%20Object%20Reference) (OtherActor :type Actor%20Object%20Reference) (OtherComp :type Primitive%20Component%20Object%20Reference) (OtherBodyIndex :type Integer))
  (Utilities|Casting|CastToSideScrollerCharacter OtherActor)
  (Variables|Default|SetCharacterInVolume false))

(event EventTick
  (params (DeltaSeconds :type Float%20%28single-precision%29))
  (if (Variables|Default|GetCharacterInVolume)
    (Utilities|FlowControl|Delay (Variables|HealthChangeZoneSettings|GetHP%20Change%20Delay))
    (Variables|/Game/BLUEPRINTS_TRABAJO/SideScrollerCharacter.SideScrollerCharacter_C|SetPlayer%20Health (stale OnComponentBeginOverlap(Box) _asside_scroller_character) (+ (Variables|/Game/BLUEPRINTS_TRABAJO/SideScrollerCharacter.SideScrollerCharacter_C|GetPlayer%20Health (stale OnComponentBeginOverlap(Box) _asside_scroller_character)) (Variables|HealthChangeZoneSettings|GetChange%20in%20Health)))))

(fn ConstructionScript)